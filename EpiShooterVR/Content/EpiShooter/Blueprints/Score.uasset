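; Score is a Blueprint that displays the player's score through a widget component in EpiShooter.
; On BeginPlay it casts the first player pawn to VRPawn and caches the reference.
; Every Tick it casts the component's widget to ScoreWidget and sets the ScoreNumber text from the pawn's Score, polling the value rather than reacting to changes.
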(event EventBeginPlay
  (bind _asvrpawn (Utilities|Casting|CastToVRPawn (Game|Player|GetPlayerPawn 0)))
  (Variables|Default|SetVRPawn _asvrpawn))

(event EventTick
  (params (DeltaSeconds :type Float%20%28single-precision%29))
  (bind _asscore_widget (Utilities|Casting|CastToScoreWidget (UserInterface|GetWidget (Variables|Default|GetScoreWidget))))
  (Rendering|Components|TextRender|SetText (Variables|/Game/EpiShooter/Blueprints/ScoreWidget.ScoreWidget_C|GetScoreNumber _asscore_widget) (Utilities|Text|ToText(Integer) (Variables|/Game/EpiShooter/Blueprints/VRPawn.VRPawn_C|GetScore (Variables|Default|GetVRPawn)))))

(fn ConstructionScript)