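; TheDwarf is an enemy Blueprint in EpiShooter that is destroyed after absorbing a set number of hits.
; Any actor overlap counts as a hit, with no check on the overlapping actor, and calls TakeHit.
; TakeHit decrements RemainingHits and destroys the actor when CanDie reports the count at zero or below.
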(event EventBeginPlay)

(event Collision|EventActorBeginOverlap
  (params (OtherActor :type Actor%20Object%20Reference))
  (CallFunction|TakeHit))

(event EventTick
  (params (DeltaSeconds :type Float%20%28single-precision%29)))

(fn ConstructionScript)

(fn CanDie
  (params (Health :type Integer))
  (return (<= Health 0)))

(fn TakeHit
  (bind _result (Math|Integer|DecrementInt (Variables|Default|GetRemaining%20Hits))
    (:%20%20
      (bind _output_get (Variables|Default|SetRemaining%20Hits _result))
      (bind _can_die (CallFunction|CanDie _output_get))
      (if _can_die
        (Actor|DestroyActor)))))