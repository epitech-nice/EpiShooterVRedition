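; Shootable enemy for a VR shooter that circles the EnemySpawn actor at its starting horizontal distance.
; Tick advances the orbit angle by a fixed per-frame step, seeded at BeginPlay from its position relative to world origin.
; Projectile overlaps reduce remaining hits; death hides the sphere, fires a material-matched explosion and updates the VRPawn's score.
; Once hidden, it destroys itself when the auto-destroying explosion becomes invalid.
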(event EventBeginPlay
  ;[1 1 1] Get origin X and Y pos of Enemy Spawner and get the horizontal distance (radius) between the enemy and its spawner
  (bind _returnvalue (Actor|GetActorOfClass "/Game/EpiShooter/Blueprints/Enemies/EnemySpawn.EnemySpawn_C"))
  (Variables|Default|SetDistance (Transformation|GetHorizontalDistanceTo _returnvalue))
  (Variables|Default|SetOriginX (.X (Class|KismetMathLibrary|BreakVector3f (Transformation|GetWorldLocation (Variables|/Game/EpiShooter/Blueprints/Enemies/EnemySpawn.EnemySpawn_C|GetDefaultSceneRoot _returnvalue)))))
  (Variables|Default|SetOriginY (.Y (Class|KismetMathLibrary|BreakVector3f (Transformation|GetWorldLocation (Variables|/Game/EpiShooter/Blueprints/Enemies/EnemySpawn.EnemySpawn_C|GetDefaultSceneRoot _returnvalue)))))
  (bind _angle (CallFunction|GetAngleBetweenTwoVectors (Transformation|GetWorldLocation (Variables|Default|GetDefaultSceneRoot)) "0, 0, 0"))
  (Variables|Default|SetAngle _angle)
  (Class|NiagaraComponent|SetVariableMaterial (Variables|Default|GetDeathExplosion) "Material" (Rendering|Material|GetMaterial (Variables|Default|GetSphere) 0)))

(event Collision|EventActorBeginOverlap
  (params (OtherActor :type Actor%20Object%20Reference))
  (CallFunction|TakeHit OtherActor))

(event EventTick
  (params (DeltaSeconds :type Float%20%28single-precision%29))
  ;[0.8685 0.6 1] Check if sphere is visible (don't move it when hidden)
  (if (Rendering|IsVisible (Variables|Default|GetSphere))
    ;[1 1 1] Set new position of the enemy
    (Transformation|SetWorldLocation (Variables|Default|GetDefaultSceneRoot) (Math|Vector|MakeVector (+ (Variables|Default|GetOriginX) (* (Math|Trig|Cos(Radians) (Math|Trig|DegreesToRadians (Variables|Default|GetAngle))) (Variables|Default|GetDistance))) (+ (Variables|Default|GetOriginY) (* (Math|Trig|Sin(Radians) (Math|Trig|DegreesToRadians (Variables|Default|GetAngle))) (Variables|Default|GetDistance))) (.Z (Class|KismetMathLibrary|BreakVector3f (Transformation|GetWorldLocation (Variables|Default|GetDefaultSceneRoot))))) false false)
    (Transformation|SetWorldLocation (Variables|Default|GetSphere) (Math|Vector|MakeVector (+ (Variables|Default|GetOriginX) (* (Math|Trig|Cos(Radians) (Math|Trig|DegreesToRadians (Variables|Default|GetAngle))) (Variables|Default|GetDistance))) (+ (Variables|Default|GetOriginY) (* (Math|Trig|Sin(Radians) (Math|Trig|DegreesToRadians (Variables|Default|GetAngle))) (Variables|Default|GetDistance))) (.Z (Class|KismetMathLibrary|BreakVector3f (Transformation|GetWorldLocation (Variables|Default|GetDefaultSceneRoot))))) false false)
    ;[1 1 1] Increase angle for the next computation
    (Variables|Default|SetAngle (+ (Variables|Default|GetAngle) 0.5))
    (else
      ;[1 0.14 0.14] Destroy enemy when sphere is hidden and explosion has ended
      (if (not (Utilities|IsValid (Variables|Default|GetDeathExplosion)))
        (Actor|DestroyActor)))))

(fn ConstructionScript)

(fn CanDie
  (params (Health :type Integer))
  (return (<= Health 0)))

(fn TakeHit
  (params (Other%20actor :type Actor%20Object%20Reference))
  (bind _deathexplosion (Variables|Default|GetDeathExplosion))
  ;[1 1 1] Check if collider is a projectile (if not, it will be ignored)
  (if (== (Utilities|GetClass Other%20actor) "/Game/EpiShooter/Blueprints/Projectile.Projectile_C")
    ;[1 1 1] Remove one to the health of the enemy
    (bind _result (Math|Integer|DecrementInt (Variables|Default|GetRemaining%20Hits))
      (:%20%20
        (bind _output_get (Variables|Default|SetRemaining%20Hits _result))
        ;[1 1 1] Check if enemy health is <= 0
        (bind _can_die (CallFunction|CanDie _output_get))
        (if _can_die
          ;[1 1 1] Comment
          (Rendering|SetVisibility (Variables|Default|GetSphere) false false)
          (Components|Activation|Activate _deathexplosion false)
          (Class|NiagaraComponent|SetAutoDestroy _deathexplosion true)
          ;[1 1 1] Increment player score
          (bind _asvrpawn (Utilities|Casting|CastToVRPawn (Game|Player|GetPlayerPawn 0)))
          (bind _result_2 (Math|Integer|IncrementInt (Variables|/Game/EpiShooter/Blueprints/VRPawn.VRPawn_C|GetScore _asvrpawn))
            (:%20%20
              (Variables|/Game/EpiShooter/Blueprints/VRPawn.VRPawn_C|SetScore _asvrpawn _result_2)
              (Default|EnemyDeath _asvrpawn))))))))

(fn GetAngleBetweenTwoVectors
  (params (Vector%20A :type Vector) (Vector%20B :type Vector))
  (bind _returnvalue (Class|KismetMathLibrary|VectorNormal2D Vector%20B 0.0001))
  (bind _returnvalue_2 (Class|KismetMathLibrary|VectorNormal2D Vector%20A 0.0001))
  (bind (_x _y) (Class|KismetMathLibrary|BreakVector3f _returnvalue))
  (bind (_x_2 _y_2) (Class|KismetMathLibrary|BreakVector3f _returnvalue_2))
  (bind _returnvalue_3 (Class|KismetMathLibrary|DegAtan2 _y_2 _x_2))
  (bind _returnvalue_4 (Class|KismetMathLibrary|DegAtan2 _y _x))
  (bind _returnvalue_5 (- _returnvalue_4 _returnvalue_3))
  (return (Math|Float|SelectFloat (+ _returnvalue_5 3.6e+02) _returnvalue_5 (< _returnvalue_5 0.0))))